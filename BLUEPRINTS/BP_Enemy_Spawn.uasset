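; BP_Enemy_Spawn is a moving enemy spawner that keys off the player's score in RUNNERGameMode.
; Each Tick it moves along its normalized Direction at Speed, scaled by delta time, without sweeping.
; It then reads CurrentPoints from the game mode and spawns an Enemy at its root transform on every frame that value equals exactly 1000, with no one-shot guard.
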(event EventBeginPlay)

(event Collision|EventActorBeginOverlap
  (params (OtherActor :type Actor%20Object%20Reference)))

(event EventTick
  (params (DeltaSeconds :type Float%20%28single-precision%29))
  (bind _defaultsceneroot (Variables|Default|GetDefaultSceneRoot))
  (bind _returnvalue (Transformation|GetWorldTransform _defaultsceneroot))
  (bind (_location _rotation _scale) (Math|Transform|BreakTransform _returnvalue))
  (Transformation|SetActorTransform (Math|Transform|MakeTransform (+ (* (Math|Vector|Normalize (Variables|Default|Getdirection)) (* (Utilities|Time|GetWorldDeltaSeconds) (Variables|Default|Getspeed))) _location) _rotation _scale))
  (bind _asrunnergame_mode (Utilities|Casting|CastToRUNNERGameMode (Game|GetGameMode)))
  (bind _output_get (Variables|/Game/BLUEPRINTS/RUNNERGameMode.RUNNERGameMode_C|SetCurrent%20Points _asrunnergame_mode (Variables|/Game/BLUEPRINTS/RUNNERGameMode.RUNNERGameMode_C|GetCurrent%20Points _asrunnergame_mode)))
  (if (== _output_get 1000)
    (Game|SpawnActorfromClass "/Game/BLUEPRINTS/Enemy.Enemy_C" (Transformation|GetWorldTransform (Variables|Default|GetDefaultSceneRoot)) "Undefined" 0 0)))

(fn ConstructionScript)